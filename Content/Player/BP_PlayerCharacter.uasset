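; Player character Blueprint with a first-person body mesh, FPSBody, whose upper arm bones the construction script hides.
; Tick prints the control rotation and the movement component's crouch intent every frame as debug output.
; An unconnected FlipFlop holds a crouch toggle that would set the AnimBlueprint's Crouching flag and shift FPSBody vertically to compensate, but it never runs.
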(event EventBeginPlay)

(event Collision|EventActorBeginOverlap
  (params (OtherActor :type Actor%20Object%20Reference)))

(event EventTick
  (params (DeltaSeconds :type Float%20%28single-precision%29))
  (Development|PrintString (Utilities|String|ToString(Rotator) (Pawn|GetControlRotation (Pawn|GetController) :!class /Script/Engine.Controller)) true true "(R=0.000000,G=0.660000,B=1.000000,A=1.000000)" 0.0)
  (Development|PrintString (Utilities|String|ToString(Boolean) (Variables|/Script/Engine.CharacterMovementComponent|GetbWantsToCrouch (Variables|Character|GetCharacterMovement))) true true "(R=0.000000,G=0.660000,B=1.000000,A=1.000000)" 0.0))

(fn ConstructionScript
  (Components|SkinnedMesh|HideBonebyName (Variables|Default|GetFPSBody) "upperarm_l" "PBO_None")
  (Components|SkinnedMesh|HideBonebyName (Variables|Default|GetFPSBody) "upperarm_r" "PBO_None"))